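; Player actor for a King of Tokyo-style monster board game, tracking one player's life, energy and stars.
; On BeginPlay, if the game instance marks this player as playing, it spawns the selected monster's scorecard and token, then initializes stats.
; Functions adjust stats, flag death, open VictoryScreen at the winning score, and move the token between TokyoCity and its marker.
; Attack is empty and damage calculation is a pass-through.
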(event `self.ReceiveTick`
  (params (DeltaSeconds :type "Float (single-precision)")))

(event `self.ReceiveBeginPlay`
  ;[1 1 1] Find out if the character is in the game (isPlaying) and activate only if he is
  (bind _asnew_game_instance (cast `/Game/My_Content/Blueprints/NewGameInstance` (`GameplayStatics.GetGameInstance`)))
  ;[1 1 1] Spawns the appropriate character score card
  (if (`KismetArrayLibrary.Array_Get` (`/Game/My_Content/Blueprints/NewGameInstance.isPlaying` _asnew_game_instance) (`self.playerNum`))
    (bind _newvar_0 (`self.setScorecard`))
    (`|SpawnActorFromClass` _newvar_0 (`self.GetTransform` self) "Undefined" "OverrideRootScale")
    ;[1 1 1] Creates the token needed for marking the king spot
    (bind _outactors (`GameplayStatics.GetAllActorsOfClass` "/Game/My_Content/Blueprints/marker.marker_C"))
    (bind _output_get (set `self.marker` (`KismetArrayLibrary.Array_Get` _outactors (`self.playerNum`))))
    (bind _newvar_0_2 (`self.setToken`))
    (bind _returnvalue (`|SpawnActorFromClass` _newvar_0_2 (`KismetMathLibrary.Conv_VectorToTransform` (`self.K2_GetActorLocation` _output_get)) "Undefined" "OverrideRootScale"))
    (set `self.token` _returnvalue)
    ;[1 1 1] Set startings values. Life 10, Energy 0, Stars 0
    (set `self.lifePoints` 5)
    (set `self.energy` 0)
    (set `self.stars` 0)))

(fn `Attack`
  (params (NewParam :type Integer)))

(fn `calculateDamage`
  (params (BaseDamage :type Integer) (isKing :type Boolean))
  (returns (FinalDamage :type Integer) (isFleeing :type Boolean))
  (return BaseDamage false))

(fn `dieResults`
  (locals (die_tally :type "Array of Integer"))
  ;[1 1 1] Comment
  (bind _asnew_game_instance (cast `/Game/My_Content/Blueprints/NewGameInstance` (`GameplayStatics.GetGameInstance`)))
  (for (_array_element _array_index) (`/Game/My_Content/Blueprints/NewGameInstance.diceResults` _asnew_game_instance)
    (`KismetArrayLibrary.Array_Set` (`local.die_tally`) _array_index (+ _array_element 1))))

(fn `gainEnergy`
  (params (NewParam :type Integer))
  (set `self.energy` (+ (`self.energy`) NewParam)))

(fn `Heal`
  (params (NewParam :type Integer))
  (bind _returnvalue (+ (`self.lifePoints`) NewParam))
  (if (>= _returnvalue 10)
    (set `self.lifePoints` 10)
    (else
      (set `self.lifePoints` _returnvalue))))

(fn `Hurt`
  (params (NewParam :type Integer))
  (returns (Kill :type Boolean))
  (bind _output_get (set `self.lifePoints` (- (`self.lifePoints`) NewParam)))
  (if (<= _output_get 0)
    (set `self.isDead` true)
    (return true)
    (else
      (return (`self.isDead`)))))

(fn `Score`
  (params (NewParam :type Integer))
  (locals (WinningScore :type Integer :default 20))
  (bind _returnvalue (+ (`self.stars`) NewParam))
  (if (<= _returnvalue 0)
    (set `self.stars` 0)
    (else
      (bind _output_get (set `self.stars` _returnvalue))
      (if (>= _output_get (`local.WinningScore`))
        (bind _asnew_game_instance (cast `/Game/My_Content/Blueprints/NewGameInstance` (`GameplayStatics.GetGameInstance`)))
        (set `/Game/My_Content/Blueprints/NewGameInstance.WinningPlayer` (`self.playerNum`) _asnew_game_instance)
        (`GameplayStatics.OpenLevel` "VictoryScreen")))))

(fn `setScorecard`
  (returns (NewVar_0 :type "Actor Class Reference"))
  ;[1 1 1] Looks at the selected monster and sets the sprite to the matching score card
  (bind _asnew_game_instance (cast `/Game/My_Content/Blueprints/NewGameInstance` (`GameplayStatics.GetGameInstance`))
    (:`then`
      (`|MultiGate` false false (`KismetArrayLibrary.Array_Get` (`/Game/My_Content/Blueprints/NewGameInstance.Monsters` _asnew_game_instance) (`self.playerNum`))
        (:`Out 1`
          (bind _output_get (set `self.scorecard_sprite` "/Game/My_Content/Textures/Characters/Scoreboards/Alienoid_Sprite_Blueprint.Alienoid_Sprite_Blueprint_C"))
          (return _output_get))
        (:`Out 2`
          (bind _output_get_2 (set `self.scorecard_sprite` "/Game/My_Content/Textures/Characters/Scoreboards/CyberBunny_Sprite_Blueprint.CyberBunny_Sprite_Blueprint_C"))
          (return _output_get_2))
        (:`Out 3`
          (bind _output_get_3 (set `self.scorecard_sprite` "/Game/My_Content/Textures/Characters/Scoreboards/Gigazaur_Sprite_Blueprint.Gigazaur_Sprite_Blueprint_C"))
          (return _output_get_3))
        (:`Out 4`
          (bind _output_get_4 (set `self.scorecard_sprite` "/Game/My_Content/Textures/Characters/Scoreboards/Kraken_Sprite_Blueprint.Kraken_Sprite_Blueprint_C"))
          (return _output_get_4))
        (:`Out 5`
          (bind _output_get_5 (set `self.scorecard_sprite` "/Game/My_Content/Textures/Characters/Scoreboards/MekaDragon_Sprite_Blueprint.MekaDragon_Sprite_Blueprint_C"))
          (return _output_get_5))
        (:`Out 6`
          (bind _output_get_6 (set `self.scorecard_sprite` "/Game/My_Content/Textures/Characters/Scoreboards/TheKing_Sprite_Blueprint.TheKing_Sprite_Blueprint_C"))
          (return _output_get_6))))
    (:`CastFailed`
      (return null))))

(fn `setToken`
  (returns (NewVar_0 :type "Actor Class Reference"))
  ;[1 1 1] Looks at the selected monster and sets the sprite to the matching score card
  (bind _asnew_game_instance (cast `/Game/My_Content/Blueprints/NewGameInstance` (`GameplayStatics.GetGameInstance`))
    (:`then`
      (`|MultiGate` false false (`KismetArrayLibrary.Array_Get` (`/Game/My_Content/Blueprints/NewGameInstance.Monsters` _asnew_game_instance) (`self.playerNum`))
        (:`Out 0`
          _)
        (:`Out 1`
          _)
        (:`Out 2`
          (bind _output_get (set `self.token_sprite` "/Game/My_Content/Textures/Characters/Tokens/CyberBunny_token_bp.CyberBunny_token_bp_C"))
          (return _output_get))
        (:`Out 3`
          (bind _output_get_2 (set `self.token_sprite` "/Game/My_Content/Textures/Characters/Tokens/Gigasaur_token_bp.Gigasaur_token_bp_C"))
          (return _output_get_2))
        (:`Out 4`
          (bind _output_get_3 (set `self.token_sprite` "/Game/My_Content/Textures/Characters/Tokens/Kraken_token_bp.Kraken_token_bp_C"))
          (return _output_get_3))
        (:`Out 5`
          (bind _output_get_4 (set `self.token_sprite` "/Game/My_Content/Textures/Characters/Tokens/MekaDragon_token_bp.MekaDragon_token_bp_C"))
          (return _output_get_4))
        (:`Out 6`
          (bind _output_get_5 (set `self.token_sprite` "/Game/My_Content/Textures/Characters/Tokens/TheKing_token_bp.TheKing_token_bp_C"))
          (return _output_get_5)))
      (bind _output_get_6 (set `self.token_sprite` "/Game/My_Content/Textures/Characters/Tokens/Alienoid_token_bp.Alienoid_token_bp_C"))
      (return _output_get_6))
    (:`CastFailed`
      (return (`self.token_sprite`)))))

(fn `tokenKing`
  (locals (NewLocalVar_0 :type "Actor Object Reference"))
  (`self.K2_SetActorLocation` (`self.token`) (`self.K2_GetActorLocation` (`self.TokyoCity`)) false false))

(fn `tokenReturn`
  (`self.K2_SetActorLocation` (`self.token`) (`self.K2_GetActorLocation` (`self.marker`)) false false))

(fn `UserConstructionScript`)