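; Physics-driven six-sided game die with heart, 1, 2, 3, claw and lightning faces.
; BeginRoll, unless locked, teleports it to a launch point with a random facing and impulse; Tick detects rest, with a timeout for stuck rolls.
; The highest side component sets the result in NewGameInstance's DiceResults, then Tick pulls the die to StartLocation and eases its rotation square.
; Per-face dynamic materials let Glow functions light the rolled face.
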(event `self.ReceiveActorBeginOverlap`
  (params (OtherActor :type "Actor Object Reference")))

(event `self.ReceiveTick`
  (params (DeltaSeconds :type "Float (single-precision)"))
  (bind _returnvalue (`self.K2_GetActorRotation`))
  (bind _startlocation (`self.startLocation`))
  (bind _targetrotation (`self.targetRotation`))
  (bind _staticmeshcomponent (`self.StaticMeshComponent`))
  (bind _returnvalue_2 (`self.K2_GetActorLocation` self))
  ;[1 1 1] only run if it's moving.
  (if (`self.isMoving`)
    ;[1 1 1] Prevents the check from going off too soon.
    (bind _output_get (set `self.rollTimer` (- (`self.rollTimer`) DeltaSeconds)))
    (if (< _output_get 3.0)
      ;[1 1 1] Checks for when the die is done moving, by checking it's velocity.  Triggers end roll function once it is no longer moving
      (bind _returnvalue_3 (`PrimitiveComponent.GetPhysicsLinearVelocity` _staticmeshcomponent "None"))
      (if (== _returnvalue_3 (0.0 0.0 0.0) :`ErrorTolerance` 0.001)
        (`self.StopRoll` :!label _label)
        (else
          ;;[1 1 1] A physics glitch can cause a die to never stop rolling.  If a die rolls too long, the timer will force it.
          (if (<= (`self.rollTimer`) 0.0)
            (goto _label)))))
    (else
      ;[1 1 1] When the die has stopped moving, kill any residual movement.
      (if (not (== _returnvalue_2 _startlocation))
        (`PrimitiveComponent.SetPhysicsLinearVelocity` _staticmeshcomponent (- _startlocation _returnvalue_2) false "None"))
      ;[1 1 1] Makes sure the right side of the die faces up.
      ;;[1 1 1] If too much time passes, set directly to the right facing
      (bind _output_get_2 (set `self.spinTimer` (- (`self.spinTimer`) DeltaSeconds)))
      ;;[1 1 1] Once the die is close enough to the right facing, lock it in place
      (if (< _output_get_2 0.0)
        ;;[1 1 1] Lock position so nothing can move it out of place
        (`self.K2_SetActorRotation` _targetrotation true :!label _label_2)
        (elif (== _returnvalue _targetrotation :`ErrorTolerance` 10.0)
          (goto _label_2)
          (else
            (`self.K2_SetActorRotation` (`KismetMathLibrary.RInterpTo` _returnvalue _targetrotation (`GameplayStatics.GetWorldDeltaSeconds`) 1.0) true))))
      (`PrimitiveComponent.SetPhysicsAngularVelocity` (`self.StaticMeshComponent`) (0.0 0.0 0.0) false "None"))))

(event `self.ReceiveBeginPlay`)

(fn `BeginRoll`
  (locals (start_rot :type "Rotator Structure" :default (struct :`Roll` 90.0)))
  ;[1 1 1] Randomly determines the starting facing of the die, to ensure fairness.
  (if (not (`self.isLocked`))
    (switch `int` (`KismetMathLibrary.RandomIntegerInRange` 0 5)
      (:`0`
        (set `local.start_rot` (`self.rot_heart`)))
      (:`1`
        (set `local.start_rot` (`self.rot_1`)))
      (:`2`
        (set `local.start_rot` (`self.rot_2`)))
      (:`3`
        (set `local.start_rot` (`self.rot_3`)))
      (:`4`
        (set `local.start_rot` (`self.rot_lightning`)))
      (:`5`
        (set `local.start_rot` (`self.rot_claw`))))
    ;[1 1 1] Move back to start position in the air
    (`self.K2_TeleportTo` (`self.launchLocation`) (`local.start_rot`))
    ;[1 1 1] Gives a random spin to the dice
    (`PrimitiveComponent.AddImpulse` (`self.StaticMeshComponent`) (* (`KismetMathLibrary.MakeVector` (`KismetMathLibrary.RandomFloatInRange` -10.0 10.0) (`KismetMathLibrary.RandomFloatInRange` -10.0 10.0)) 10) "None" false)
    ;[1 1 1] Sets variables to control the end of the roll
    (set `self.isMoving` true) ; Makrs isMoving as true
    (set `self.rollTimer` 5.0) ; sets the roll TImer
    (set `self.spinTimer` 5.0)))

(fn `Facing`
  (bind _indexofmaxvalue (`KismetMathLibrary.MaxOfFloatArray` (`|MakeArray` (.z (`SceneComponent.K2_GetComponentLocation` (`self.sideHeart`))) (.z (`SceneComponent.K2_GetComponentLocation` (`self.side1`))) (.z (`SceneComponent.K2_GetComponentLocation` (`self.side2`))) (.z (`SceneComponent.K2_GetComponentLocation` (`self.side3`))) (.z (`SceneComponent.K2_GetComponentLocation` (`self.sideClaw`))) (.z (`SceneComponent.K2_GetComponentLocation` (`self.sideLightning`))))))
  (bind _asnew_game_instance (cast `/Game/My_Content/Blueprints/NewGameInstance` (`GameplayStatics.GetGameInstance`)))
  (`KismetArrayLibrary.Array_Set` (`/Game/My_Content/Blueprints/NewGameInstance.diceResults` _asnew_game_instance) (`self.dieNumber`) _indexofmaxvalue)
  (switch `int` _indexofmaxvalue
    (:`0`
      (set `self.targetRotation` (`self.rot_heart`)))
    (:`1`
      (set `self.targetRotation` (`self.rot_1`)))
    (:`2`
      (set `self.targetRotation` (`self.rot_2`)))
    (:`3`
      (set `self.targetRotation` (`self.rot_3`)))
    (:`4`
      (set `self.targetRotation` (`self.rot_claw`)))
    (:`5`
      (set `self.targetRotation` (`self.rot_lightning`)))))

(fn `Glow_1`
  (params (Target_glow :type "Float (double-precision)") (Die_Results :type "Array of Integer"))
  (if (== (`KismetArrayLibrary.Array_Get` Die_Results (`self.dieNumber`)) 1)
    (`MaterialInstanceDynamic.SetScalarParameterValue` (`self.glow_score1`) "Emmisive_Strength" Target_glow)))

(fn `Glow_2`
  (params (Target_glow :type "Float (double-precision)") (Die_Results :type "Array of Integer"))
  (if (== (`KismetArrayLibrary.Array_Get` Die_Results (`self.dieNumber`)) 2)
    (`MaterialInstanceDynamic.SetScalarParameterValue` (`self.glow_score2`) "Emmisive_Strength" Target_glow)))

(fn `Glow_3`
  (params (Target_glow :type "Float (double-precision)") (Die_Results :type "Array of Integer"))
  (if (== (`KismetArrayLibrary.Array_Get` Die_Results (`self.dieNumber`)) 3)
    (`MaterialInstanceDynamic.SetScalarParameterValue` (`self.glow_score3`) "Emmisive_Strength" Target_glow)))

(fn `Glow_c`
  (params (Target_glow :type "Float (double-precision)") (Die_Results :type "Array of Integer"))
  (if (== (`KismetArrayLibrary.Array_Get` Die_Results (`self.dieNumber`)) 4)
    (`MaterialInstanceDynamic.SetScalarParameterValue` (`self.glow_claw`) "Emmisive_Strength" Target_glow)))

(fn `Glow_h`
  (params (Target_glow :type "Float (double-precision)") (Die_Results :type "Array of Integer"))
  (if (== (`KismetArrayLibrary.Array_Get` Die_Results (`self.dieNumber`)) 0)
    (`MaterialInstanceDynamic.SetScalarParameterValue` (`self.glow_heart`) "Emmisive_Strength" Target_glow)))

(fn `Glow_l`
  (params (Target_glow :type "Float (double-precision)") (Die_Results :type "Array of Integer"))
  (if (== (`KismetArrayLibrary.Array_Get` Die_Results (`self.dieNumber`)) 5)
    (`MaterialInstanceDynamic.SetScalarParameterValue` (`self.glow_lightning`) "Emmisive_Strength" Target_glow)))

(fn `StopRoll`
  (set `self.isMoving` false)
  (`self.Facing`))

(fn `UserConstructionScript`
  (bind _returnvalue (`PrimitiveComponent.CreateDynamicMaterialInstance` (`self.sideHeart`) 0 "/Game/My_Content/SpecialEffects/Emissive_Material_dH_Inst.Emissive_Material_dH_Inst"))
  (set `self.glow_heart` _returnvalue)
  (bind _returnvalue_2 (`PrimitiveComponent.CreateDynamicMaterialInstance` (`self.side1`) 0 "/Game/My_Content/SpecialEffects/Emissive_Material_d1.Emissive_Material_d1"))
  (set `self.glow_score1` _returnvalue_2)
  (bind _returnvalue_3 (`PrimitiveComponent.CreateDynamicMaterialInstance` (`self.side2`) 0 "/Game/My_Content/SpecialEffects/Emissive_Material_d2.Emissive_Material_d2"))
  (set `self.glow_score2` _returnvalue_3)
  (bind _returnvalue_4 (`PrimitiveComponent.CreateDynamicMaterialInstance` (`self.side3`) 0 "/Game/My_Content/SpecialEffects/Emissive_Material_d3.Emissive_Material_d3"))
  (set `self.glow_score3` _returnvalue_4)
  (bind _returnvalue_5 (`PrimitiveComponent.CreateDynamicMaterialInstance` (`self.sideClaw`) 0 "/Game/My_Content/SpecialEffects/Emissive_Material_dC.Emissive_Material_dC"))
  (set `self.glow_claw` _returnvalue_5)
  (bind _returnvalue_6 (`PrimitiveComponent.CreateDynamicMaterialInstance` (`self.sideLightning`) 0 "/Game/My_Content/SpecialEffects/Emissive_Material_dL.Emissive_Material_dL"))
  (set `self.glow_lightning` _returnvalue_6))